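; PredictionText_BP is a head-locked text display that shows hand-data prediction results to the player.
; On BeginPlay it caches its Text_Widget, attaches its root to the HandsPawn_BP camera and binds to the pawn's HandDataSender events.
; Prediction results (class and accuracy) and test-state strings are stored separately, and either update rewrites the prompt with both combined.
; A HandTypeToString helper maps hand type to text but is not called here.
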(event `self.ReceiveBeginPlay`
  (bind _astext_widget (cast `/Game/HandsML/Blueprints/Text_Widget` (`WidgetComponent.GetUserWidgetObject` (`self.Widget`))))
  (set `self.propmtWidget` _astext_widget)
  (bind _ashands_pawn_bp (cast `/Game/HandsML/Blueprints/HandsPawn_BP` (`GameplayStatics.GetPlayerPawn` 0)))
  (`SceneComponent.K2_AttachToComponent` (`self.DefaultSceneRoot`) (`/Game/HandsML/Blueprints/HandsPawn_BP.PlayerCamera` _ashands_pawn_bp) "None" "KeepRelative" "KeepRelative" "KeepRelative" true)
  (bind _handdatasender (`/Game/HandsML/Blueprints/HandsPawn_BP.HandDataSender` _ashands_pawn_bp))
  (add `HandDataSender.OnPredictionResult` _handdatasender (delegate `WriteResult`))
  (add `HandDataSender.OnTest` _handdatasender (delegate `WriteState`)))

(event `WriteState`
  (params (String :type String))
  (set `self.TestStr` (`KismetTextLibrary.Conv_StringToText` String))
  (`/Game/HandsML/Blueprints/Text_Widget.SetPromptText` (`self.propmtWidget`) (`|FormatText` "{0} {1}" (`self.Result`) (`self.TestStr`)) :!label _label))

(event `WriteResult`
  (params (Class :type String) (Accuracy :type String))
  (set `self.Result` (`|FormatText` "Class: {0}; Acc: {1}" Class Accuracy))
  (goto _label))

(fn `HandTypeToString`
  (params (inType :type "EOculusHandType Enum" :default "None"))
  (returns (outType :type String))
  (switch `EOculusHandType` inType
    (:`HandLeft`
      (return "left"))
    (:`HandRight`
      (return "right"))))

(fn `UserConstructionScript`)