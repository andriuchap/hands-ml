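; HandsPawn_BP is a pawn that turns right-hand poses into action events through predictions received from HandDataSender.
; When predictions are enabled, a looping timer captures the pose and sends it to HandDataSender.
; Returned classes above a 0.9 accuracy threshold fire OnAction only when they differ from the last class, while low-confidence results reset that class.
; BeginPlay also sets floor-level tracking and fills a ClassTemporal array, unused in this graph.
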(event `self.ReceiveBeginPlay`
  (for _ (range 8)
    (`KismetArrayLibrary.Array_Add` (`self.classTemporal`) -1))
  (`HeadMountedDisplayFunctionLibrary.SetTrackingOrigin` "Floor")
  (if (`self.startPredictions`)
    (`KismetSystemLibrary.K2_SetTimerDelegate` (delegate `Start Captures`) (`self.predictionTickTime`) true)
    (add `HandDataSender.OnPredictionResult` (`self.HandDataSender`) (delegate `OnPredictionResult`))))

(event `Start Captures`
  (bind _returnvalue (`HandsMLFunctionLibrary.CapturePose` (`self.RightHand`)))
  (`HandDataSender.SendHandData` (`self.HandDataSender`) _returnvalue))

(event `OnPredictionResult`
  (params (Class :type String) (Accuracy :type String))
  (bind _returnvalue (`KismetStringLibrary.Conv_StringToInt` Class))
  (if (> (`KismetStringLibrary.Conv_StringToDouble` Accuracy) 0.9)
    (if (!= _returnvalue (`self.lastClass`))
      (bind _output_get (set `self.lastClass` _returnvalue))
      (`self.OnAction` _output_get))
    (else
      (set `self.lastClass` -1))))

(fn `UserConstructionScript`)