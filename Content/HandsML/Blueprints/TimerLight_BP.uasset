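; TimerLight_BP is a countdown indicator that flashes a light and beeps while a SnapShotter's snapshot timer runs.
; It binds to the SnapShotter's timer-started, snapshot and cancelled events, starting the beep cycle on the first and silencing it on the others.
; Chained one-shot timers toggle audio and a dynamic material's Strength, shrinking each wait by a decay factor down to the beep duration, so beeps accelerate.
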(event `CancelBeeping`
  (`AudioComponent.Stop` (`self.beepAudio`) :!label _label)
  (`MaterialInstanceDynamic.SetScalarParameterValue` (`self.lightMaterial`) "Strength" 0.0)
  (`KismetSystemLibrary.K2_ClearAndInvalidateTimerHandle` (`self.beepTimer`)))

(event `self.ReceiveBeginPlay`
  (bind _snapshotter (`self.snapShotter`))
  (bind _returnvalue (`PrimitiveComponent.CreateDynamicMaterialInstance` (`self.StaticMeshComponent`) 0 "/Game/HandsML/M_LightDynamic.M_LightDynamic" "None"))
  (bind _output_get (set `self.lightMaterial` _returnvalue))
  (`MaterialInstanceDynamic.SetScalarParameterValue` _output_get "Strength" 0.0)
  (`/Engine/EditorBlueprintResources/StandardMacros.IsValid` _snapshotter
    (:`Is Valid`
      (add `/Game/HandsML/Blueprints/HandSnapshotter_BP.OnSnapshotTimerStarted` _snapshotter (delegate `SnapshotTimerStarted`))
      (add `/Game/HandsML/Blueprints/HandSnapshotter_BP.OnSnapshot` _snapshotter (delegate `InterruptBeeping`))
      (add `/Game/HandsML/Blueprints/HandSnapshotter_BP.OnSnapshotCancelled` _snapshotter (delegate `CancelBeeping`)))))

(event `InterruptBeeping`
  (goto _label))

(event `SnapshotTimerStarted`
  (params (class :type String) (handType :type "EOculusHandType Enum" :default "None"))
  (bind _output_get (set `self.beepCurrentWaitTime` (`self.beepBaseWaitTime`)))
  (bind _returnvalue (`KismetSystemLibrary.K2_SetTimerDelegate` (delegate `WaitForBeepFinished`) _output_get))
  (set `self.beepTimer` _returnvalue))

(event `WaitForBeepFinished`
  (`self.Beep`))

(event `Beep`
  (`MaterialInstanceDynamic.SetScalarParameterValue` (`self.lightMaterial`) "Strength" 10.0)
  (`AudioComponent.Play` (`self.beepAudio`) 0.0)
  (bind _returnvalue (`KismetSystemLibrary.K2_SetTimerDelegate` (delegate `FinishBeep`) (`self.beepDuration`)))
  (set `self.beepTimer` _returnvalue))

(event `FinishBeep`
  (`AudioComponent.Stop` (`self.beepAudio`))
  (`MaterialInstanceDynamic.SetScalarParameterValue` (`self.lightMaterial`) "Strength" 0.0)
  (bind _output_get (set `self.beepCurrentWaitTime` (`KismetMathLibrary.FMax` (* (`self.beepCurrentWaitTime`) (`self.beepWaitTimeDecay`)) (`self.beepDuration`))))
  (bind _returnvalue (`KismetSystemLibrary.K2_SetTimerDelegate` (delegate `WaitForBeepFinished`) _output_get))
  (set `self.beepTimer` _returnvalue))

(fn `UserConstructionScript`)