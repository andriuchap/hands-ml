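; PromptText_BP is an in-world prompt that shows which hand and pose are requested when a HandShotter snapshot timer starts.
; On BeginPlay it caches the Text_Widget from its widget component and binds PromptPose to the HandShotter's OnSnapshotTimerStarted event.
; PromptPose converts the hand type to "left" or "right", formats it with the pose class and sets the widget's prompt text.
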(event `self.ReceiveBeginPlay`
  (bind _as3dtext_widget (cast `/Game/HandsML/Blueprints/Text_Widget` (`WidgetComponent.GetUserWidgetObject` (`self.Widget`))))
  (set `self.propmtWidget` _as3dtext_widget)
  (add `/Game/HandsML/Blueprints/HandSnapshotter_BP.OnSnapshotTimerStarted` (`self.handShotter`) (delegate `PromptPose`)))

(event `PromptPose`
  (params (class :type String) (handType :type "EOculusHandType Enum" :default "None"))
  (`/Game/HandsML/Blueprints/Text_Widget.SetPromptText` (`self.propmtWidget`) (`|FormatText` "Hand: {0}; Pose: {1}" (`self.HandTypeToString` handType) class)))

(fn `HandTypeToString`
  (params (inType :type "EOculusHandType Enum" :default "None"))
  (returns (outType :type String))
  (switch `EOculusHandType` inType
    (:`HandLeft`
      (return "left"))
    (:`HandRight`
      (return "right"))))

(fn `UserConstructionScript`)