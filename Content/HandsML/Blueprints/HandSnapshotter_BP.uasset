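; HandSnapshotter is an input-enabled Blueprint that captures hand bone position snapshots on a timer and writes them out.
; ToggleSnapshot starts or cancels the countdown, using timer handle validity as its running state.
; On expiry it fires a snapshot event, plays a camera sound and calls NewPosition on BonePosition.
; WriteData delegates saving to BonePosition, with audio feedback throughout and events for timer start and cancellation.
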(event `self.ReceiveBeginPlay`
  (`self.EnableInput` (`GameplayStatics.GetPlayerController` 0)))

(event `Key|K`
  (params (Key :type "Key Structure")))

(event `StartSnapshotTimer`
  (if (not (`self.IsStarted`))
    (bind _returnvalue (`KismetSystemLibrary.K2_SetTimerDelegate` (delegate `ExecuteSnapshot`) (`self.snapshotTimeout`)))
    (set `self.snapShotTimer` _returnvalue)
    (`self.OnSnapshotTimerStarted`)))

(event `ExecuteSnapshot`
  (`self.OnSnapshot`)
  (`GameplayStatics.PlaySound2D` "/Game/HandsML/CameraShot.CameraShot" 1.0 1.0 0.0 null null)
  (`/Game/HandsML/Blueprints/BonePositions_BP.NewPosition` (`self.bonePosition`)))

(event `StopSnapshotTimer`
  (if (`self.IsStarted`)
    (`KismetSystemLibrary.K2_ClearAndInvalidateTimerHandle` (`self.snapShotTimer`))
    (`self.OnSnapshotCancelled`)))

(event `ToggleSnapshot`
  (if (`self.IsStarted`)
    (`self.StopSnapshotTimer`)
    (`GameplayStatics.PlaySound2D` "/Game/HandsML/NegativeFeedback.NegativeFeedback" 1.0 1.0 0.0 null null)
    (else
      (`self.StartSnapshotTimer`)
      (`GameplayStatics.PlaySound2D` "/Game/HandsML/PositiveFeedback.PositiveFeedback" 1.0 1.0 0.0 null null))))

(event `WriteData`
  (`/Game/HandsML/Blueprints/BonePositions_BP.WriteData` (`self.bonePosition`))
  (`GameplayStatics.PlaySound2D` "/Game/HandsML/FloppyWrite.FloppyWrite" 1.0 1.0 0.0 null null))

(fn `IsStarted`
  (returns (`Is Started` :type Boolean))
  (return (`KismetSystemLibrary.K2_IsValidTimerHandle` (`self.snapShotTimer`))))

(fn `UserConstructionScript`)